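; Keyboard-flown helicopter actor with a spinning rotor and a first- or third-person view toggled by Tab.
; Q/E change rotor speed, which spins the blade and sets climb or descent around a lift threshold.
; While flying, W/S and A/D adjust persistent forward and turn speeds that also tilt the body.
; Tick applies this movement by setting transforms directly and moves the player pawn to the selected viewpoint.
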(event EventBeginPlay)

(event Collision|EventActorBeginOverlap
  (params (OtherActor :type Actor%20Object%20Reference)))

(event EventTick
  (params (DeltaSeconds :type Float%20%28single-precision%29))
  (CallFunction|SetIsFlyingVar)
  (CallFunction|SetHelicopterLocation DeltaSeconds)
  (CallFunction|SetHelicopterRotation)
  (CallFunction|SetBladeRotation)
  (CallFunction|SetPlayerLocation)
  (if (Utilities|IsFlying)
    (if (Variables|Default|GetisW)
      (Variables|Default|SetWSSpeed (Math|Float|SelectFloat 3.0 (+ (Variables|Default|GetWSSpeed) (* DeltaSeconds 1.0)) (> (+ (Variables|Default|GetWSSpeed) (* DeltaSeconds 1.0)) 3.0)))
      (elif (Variables|Default|GetisS)
        (Variables|Default|SetWSSpeed (Math|Float|SelectFloat -3.0 (- (Variables|Default|GetWSSpeed) (* DeltaSeconds 1.0)) (< (- (Variables|Default|GetWSSpeed) (* DeltaSeconds 1.0)) -3.0))))))
  (if (Utilities|IsFlying)
    (if (Variables|Default|GetisA)
      (Variables|Default|SetADSpeed (Math|Float|SelectFloat 3.0 (+ (Variables|Default|GetADSpeed) (* DeltaSeconds 1.0)) (> (+ (Variables|Default|GetADSpeed) (* DeltaSeconds 1.0)) 3.0)))
      (elif (Variables|Default|GetisD)
        (Variables|Default|SetADSpeed (Math|Float|SelectFloat -3.0 (- (Variables|Default|GetADSpeed) (* DeltaSeconds 1.0)) (< (- (Variables|Default|GetADSpeed) (* DeltaSeconds 1.0)) -3.0))))))
  (if (Variables|Default|GetisQ)
    (Variables|Default|SetMainRotorSpeed (Math|Float|SelectFloat 3e+01 (+ (Variables|Default|GetMainRotorSpeed) (* DeltaSeconds 1.0)) (> (+ (Variables|Default|GetMainRotorSpeed) (* DeltaSeconds 1.0)) 3e+01)))
    (elif (Variables|Default|GetisE)
      (Variables|Default|SetMainRotorSpeed (Math|Float|SelectFloat 0.0 (- (Variables|Default|GetMainRotorSpeed) (* DeltaSeconds 1.0)) (< (- (Variables|Default|GetMainRotorSpeed) (* DeltaSeconds 1.0)) 0.0))))))

(event Input|KeyboardEvents|Q
  (params (Key :type Key%20Structure))
  (:Pressed
    (Variables|Default|SetisQ true))
  (:Released
    (Variables|Default|SetisQ false)))

(event Input|KeyboardEvents|E
  (params (Key :type Key%20Structure))
  (:Pressed
    (Variables|Default|SetisE true))
  (:Released
    (Variables|Default|SetisE false)))

(event Input|KeyboardEvents|Tab
  (params (Key :type Key%20Structure))
  (:Pressed
    (Variables|Default|SetisThirdPerson (not (Variables|Default|GetisThirdPerson)))))

(event Input|KeyboardEvents|W
  (params (Key :type Key%20Structure))
  (:Pressed
    (Variables|Default|SetisW true))
  (:Released
    (Variables|Default|SetisW false)))

(event Input|KeyboardEvents|A
  (params (Key :type Key%20Structure))
  (:Pressed
    (Variables|Default|SetisA true))
  (:Released
    (Variables|Default|SetisA false)))

(event Input|KeyboardEvents|S
  (params (Key :type Key%20Structure))
  (:Pressed
    (Variables|Default|SetisS true))
  (:Released
    (Variables|Default|SetisS false)))

(event Input|KeyboardEvents|D
  (params (Key :type Key%20Structure))
  (:Pressed
    (Variables|Default|SetisD true))
  (:Released
    (Variables|Default|SetisD false)))

(fn ConstructionScript)

(fn SetPlayerLocation
  (bind _isthirdperson (Variables|Default|GetisThirdPerson))
  (bind _firstperson (Variables|Default|GetFirstPerson))
  (bind _root (Variables|Default|GetRoot))
  (bind _returnvalue (Transformation|GetWorldLocation _firstperson))
  (bind _returnvalue_2 (Transformation|GetWorldLocation _root))
  (Transformation|SetActorLocation (Game|Player|GetPlayerPawn 0) (Math|Vector|MakeVector (select _isthirdperson (+ (.x _returnvalue_2) (* (Math|Trig|Sin(Degrees) (Variables|Default|GetZValue)) 2e+03)) (.x _returnvalue)) (select _isthirdperson (- (.y _returnvalue_2) (* (Math|Trig|Cos(Degrees) (Variables|Default|GetZValue)) 2e+03)) (.y _returnvalue)) (select _isthirdperson (+ (.z _returnvalue_2) 1e+03) (.z _returnvalue))) false false))

(fn SetBladeRotation
  (bind _bp_blade (Variables|Default|GetBP_Blade))
  (bind _relativerotation (Variables|/Script/Engine.SceneComponent|GetRelativeRotation _bp_blade))
  (Transformation|SetRelativeRotation (Variables|Default|GetBP_Blade) (Math|Rotator|MakeRotator (.roll _relativerotation) (.pitch _relativerotation) (+ (.yaw _relativerotation) (Variables|Default|GetMainRotorSpeed))) false false))

(fn SetHelicopterRotation
  (Transformation|SetWorldRotation (Variables|Default|GetRoot) (Math|Rotator|MakeRotator (* (Variables|Default|GetWSSpeed) 1e+01) (* (Variables|Default|GetADSpeed) -1e+01) (Variables|Default|GetZValue)) false false))

(fn SetHelicopterLocation
  (params (deltaTime :type Float%20%28double-precision%29))
  (bind _root (Variables|Default|GetRoot))
  (bind _root_2 (Variables|Default|GetRoot))
  (bind _returnvalue (Transformation|GetWorldLocation _root))
  (bind _returnvalue_2 (Transformation|GetWorldLocation _root_2))
  (if (Utilities|IsFlying)
    (Transformation|SetWorldLocation (Variables|Default|GetRoot) (Math|Vector|MakeVector (+ (.x _returnvalue) (* (* (* (Variables|Default|GetWSSpeed) deltaTime) 1e+03) (Math|Trig|Sin(Degrees) (- 3.6e+02 (Variables|Default|GetZValue))))) (+ (.y _returnvalue) (* (* (* (Variables|Default|GetWSSpeed) deltaTime) 1e+03) (Math|Trig|Cos(Degrees) (Variables|Default|GetZValue)))) (.z _returnvalue)) false false)
    (Variables|Default|SetZValue (- (Variables|Default|GetZValue) (* (* (Variables|Default|GetADSpeed) deltaTime) 1e+01))))
  (if (> (Variables|Default|GetMainRotorSpeed) 15.0)
    (Transformation|SetWorldLocation (Variables|Default|GetRoot) (Math|Vector|MakeVector (.x _returnvalue_2) (.y _returnvalue_2) (+ (.z _returnvalue_2) (* (* (- (Variables|Default|GetMainRotorSpeed) 15.0) deltaTime) 1e+03))) false false :!label _label)
    (elif (Utilities|IsFlying)
      (goto _label))))

(fn SetIsFlyingVar
  (if (> (Variables|Default|GetMainRotorSpeed) 15.0)
    (Variables|Default|SetisFlyingVar true)))